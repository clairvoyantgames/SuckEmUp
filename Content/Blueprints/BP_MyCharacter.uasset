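; BP_MyCharacter is a 2D flipbook player character that runs along the X axis and jumps.
; The MoveRight axis event refreshes the animation, choosing run or idle from velocity, then applies movement input when CanWalk is true.
; Facing is handled by rotating the capsule 180 degrees by travel direction; the sprite rotation nodes are left unconnected.
; Jump input is gated by the same CanWalk flag.
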(event Custom|UpdateAnimation
  ;[1 1 1] Handle Animation
  (Sprite|SetFlipbook (Variables|Default|GetSprite) (select (> (Math|Vector|VectorLength (Transformation|GetVelocity)) 0.0) "/Game/Sprites/PlayerRunAnimation.PlayerRunAnimation" "/Game/Sprites/PlayerIdleAnimation.PlayerIdleAnimation")))

(event Input|ActionEvents|InputActionJump
  ;[1 1 1] Handle Jump
  (:Pressed
    (if (Variables|Default|GetCanWalk)
      (Character|Jump))))

(event Input|AxisEvents|InputAxisMoveRight
  (params (AxisValue :type Float%20%28single-precision%29))
  (bind _capsulecomponent (Variables|Default|GetCapsuleComponent))
  ;[1 1 1] Handle movement
  (CallFunction|UpdateAnimation)
  (if (Variables|Default|GetCanWalk)
    (if (> AxisValue 0.0)
      (Transformation|SetRelativeRotation _capsulecomponent "0, 0,0.000000" false)
      (Pawn|Input|AddMovementInput "1.000000, 0, 0" AxisValue :!label _label)
      (elif (< AxisValue 0.0)
        (Transformation|SetRelativeRotation _capsulecomponent "0,180.000000,0.000000" false)
        (goto _label)))))

(event Input|TouchEvents|InputTouch
  (params (Location :type Vector) (FingerIndex :type ETouchIndex%20Enum))
  ;[1 1 1] Handle Jump
)

(fn ConstructionScript)