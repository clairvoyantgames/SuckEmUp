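; Game mode that sets up two local players at separate PlayerStart locations when play begins.
; It gathers all PlayerStart actors, then teleports player 0's pawn to the first and creates a second local player whose pawn moves to the second.
; Each BP_PlayerCharacter also stores its start as PlayerSpawn.
; Assignment relies on the order GetAllActorsOfClass returns, with no check on the count.
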(event EventBeginPlay
  (bind _returnvalue (Game|GetPlayerController 0))
  (bind _returnvalue_2 (Pawn|GetControlledPawn _returnvalue))
  ;[1 1 1] Set Player 1 and Player 2 Location
  (Utilities|FlowControl|Sequence
    (:then_0
      (bind _outactors (Actor|GetAllActorsOfClass "/Script/Engine.PlayerStart"))
      (Variables|Default|SetPlayer%20Starts _outactors))
    (:then_1
      (bind _asbp_playercharacter_c (Utilities|Casting|CastToBP_PlayerCharacter _returnvalue_2))
      (Variables|/Game/Blueprints/BP_PlayerCharacter.BP_PlayerCharacter_C|SetPlayer%20Spawn _asbp_playercharacter_c (Utilities|Array|Get(acopy) (Variables|Default|GetPlayer%20Starts)))
      (Transformation|SetActorTransform _returnvalue_2 (Transformation|GetActorTransform (Utilities|Array|Get(acopy) (Variables|Default|GetPlayer%20Starts)))))
    (:then_2
      (bind _returnvalue_3 (Class|GameplayStatics|CreatePlayer -1))
      (bind _asbp_playercharacter_c_2 (Utilities|Casting|CastToBP_PlayerCharacter (Pawn|GetControlledPawn _returnvalue_3)))
      (Variables|/Game/Blueprints/BP_PlayerCharacter.BP_PlayerCharacter_C|SetPlayer%20Spawn _asbp_playercharacter_c_2 (Utilities|Array|Get(acopy) (Variables|Default|GetPlayer%20Starts) 1))
      (Transformation|SetActorTransform (Pawn|GetControlledPawn _returnvalue_3) (Transformation|GetActorTransform (Utilities|Array|Get(acopy) (Variables|Default|GetPlayer%20Starts) 1))))))

(fn ConstructionScript)