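; Side-scrolling player character with double jump and a levelled suck attack for pulling in and swallowing other BP_PlayerCharacter actors.
; Suck inputs grow and offset SuckCollider, and a nonzero level blocks walking and jumping.
; Tick flags overlapped players as sucked, drags itself toward others when sucked, and handles respawn cooldown.
; Swallowing kills and teleports victims to spawn, adds score, and appends a BP_SuckUmm to a linked trailing chain.
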(event Custom|Rest%20Sucks
  ;[1 1 1] Suck Inputs
  (Utilities|FlowControl|DoN (Variables|Default|GetMax%20Suck%20Level)) ; enters at Reset
)

(event Custom|Suck%20Changed
  (bind _suck_collider (Variables|Default|GetSuck%20Collider))
  (bind _is_sucked (Variables|Default|GetIs%20Sucked))
  (bind _is_stunned (Variables|Default|GetIs%20Stunned))
  (bind _relativelocation (Variables|/Script/Engine.SceneComponent|GetRelativeLocation _suck_collider))
  (bind (_x _y _z) (Math|Vector|BreakVector _relativelocation))
  ;[1 1 1] Do Suck
  (Variables|/Script/Engine.PrimitiveComponent|SetbGenerateOverlapEvents (Variables|Default|GetSuck%20Collider) (Math|Boolean|ANDBoolean (!= (Variables|Default|GetCurrent%20Suck%20Level) 0) (not _is_sucked) (not _is_stunned)))
  (Rendering|SetVisibility _suck_collider (Math|Boolean|ANDBoolean (!= (Variables|Default|GetCurrent%20Suck%20Level) 0) (not _is_sucked) (not _is_stunned)) false)
  (if (Math|Boolean|ANDBoolean (!= (Variables|Default|GetCurrent%20Suck%20Level) 0) (not _is_sucked) (not _is_stunned))
    (Utilities|FlowControl|Sequence
      (:then_0
        (Components|Sphere|SetSphereRadius (Variables|Default|GetSuck%20Collider) (+ (Variables|Default|GetCollider%20Radius) (* (Variables|Default|GetIncrease%20Rate) (Math|Conversions|ToFloat(Integer) (Variables|Default|GetCurrent%20Suck%20Level)))) true))
      (:then_1
        (Transformation|SetRelativeLocation (Variables|Default|GetSuck%20Collider) (Math|Vector|MakeVector (+ (* (Variables|Default|GetIncrease%20Rate) (Math|Conversions|ToFloat(Integer) (Variables|Default|GetCurrent%20Suck%20Level))) (Variables|Default|GetStarting%20Radius)) _y _z) false)))
    (elif (not (or _is_sucked _is_stunned))
      (Variables|Default|SetCurrent%20Suck%20Level 0)
      (CallFunction|RestSucks))))

(event Custom|Set%20Alive
  ;[1 1 1] Respawn
  (Variables|Default|SetIs%20Respawning false))

(event EventOnLanded
  (params (Hit :type Hit%20Result%20Structure%20%28by%20ref%29))
  ;[1 1 1] Double Jump
  (Utilities|FlowControl|DoN 2) ; enters at Reset
)

(event EventActorEndOverlap
  (params (OtherActor :type Actor%20Object%20Reference))
  ;[1 1 1] Released
  (Utilities|Casting|CastToBP_PlayerCharacter OtherActor)
  (Variables|Default|SetIs%20Sucked false))

(event EventTick
  (params (DeltaSeconds :type Float%20%28single-precision%29))
  (bind _returnvalue (Transformation|GetActorLocation))
  (Utilities|FlowControl|Sequence
    (:then_0
      ;[1 1 1] Suck Events
      (if (Rendering|IsVisible (Variables|Default|GetSuck%20Collider))
        (Utilities|FlowControl|Sequence
          (:then_0
            ;[1 1 1] Sucked
            (for _array_element (Collision|GetOverlappingActors (Variables|Default|GetSuck%20Collider) "/Game/Blueprints/BP_PlayerCharacter.BP_PlayerCharacter_C" :!class /Script/Engine.PrimitiveComponent)
              (bind _asbp_playercharacter_c (Utilities|Casting|CastToBP_PlayerCharacter _array_element))
              (if (and (!= _array_element self) (not (Variables|/Game/Blueprints/BP_PlayerCharacter.BP_PlayerCharacter_C|GetIs%20Respawning _asbp_playercharacter_c)))
                (Variables|/Game/Blueprints/BP_PlayerCharacter.BP_PlayerCharacter_C|SetIs%20Sucked _asbp_playercharacter_c true))))
          (:then_1
            ;[1 1 1] Swallowed
            (for _array_element_2 (Collision|GetOverlappingActors (Variables|Collision|GetCapsuleComponent) "/Game/Blueprints/BP_PlayerCharacter.BP_PlayerCharacter_C" :!class /Script/Engine.PrimitiveComponent)
              (bind _asbp_playercharacter_c_2 (Utilities|Casting|CastToBP_PlayerCharacter _array_element_2))
              (if (and (!= _array_element_2 self) (not (Variables|/Game/Blueprints/BP_PlayerCharacter.BP_PlayerCharacter_C|GetIs%20Respawning _asbp_playercharacter_c_2)))
                (Utilities|FlowControl|Sequence
                  (:then_0
                    (Variables|/Game/Blueprints/BP_PlayerCharacter.BP_PlayerCharacter_C|SetIs%20Dead _asbp_playercharacter_c_2 true))
                  (:then_1
                    (Transformation|Teleport _asbp_playercharacter_c_2 (Transformation|GetActorLocation (Variables|/Game/Blueprints/BP_PlayerCharacter.BP_PlayerCharacter_C|GetPlayer%20Spawn _asbp_playercharacter_c_2)) "0, 0, 0"))
                  (:then_2
                    (Variables|Default|SetScore (+ (Variables|Default|GetScore) 1)))
                  (:then_3
                    (bind _returnvalue_2 (Game|SpawnActorfromClass "/Game/Blueprints/BP_SuckUmm.BP_SuckUmm_C" (Transformation|GetActorTransform) true 0))
                    (if (== (Variables|Default|Getchild1) 0)
                      (Variables|/Game/Blueprints/BP_SuckUmm.BP_SuckUmm_C|SetParent%20Actor _returnvalue_2 self)
                      (Variables|Default|Setchild1 _returnvalue_2)
                      (else
                        (Variables|Default|SetobjectToCheck (Variables|Default|Getchild1))
                        (bind _asbp_suckumm_c (Utilities|Casting|CastToBP_SuckUmm (Variables|Default|GetobjectToCheck)))
                        (Variables|Default|SetobjectsChild (Variables|/Game/Blueprints/BP_SuckUmm.BP_SuckUmm_C|GetChild%20Actor _asbp_suckumm_c))
                        (while (!= (Variables|Default|GetobjectsChild) 0)
                          (bind _asbp_suckumm_c_2 (Utilities|Casting|CastToBP_SuckUmm (Variables|Default|GetobjectToCheck)))
                          (Variables|Default|SetobjectToCheck (Variables|/Game/Blueprints/BP_SuckUmm.BP_SuckUmm_C|GetChild%20Actor _asbp_suckumm_c_2))
                          (bind _asbp_suckumm_c_3 (Utilities|Casting|CastToBP_SuckUmm (Variables|Default|GetobjectToCheck)))
                          (Variables|Default|SetobjectsChild (Variables|/Game/Blueprints/BP_SuckUmm.BP_SuckUmm_C|GetChild%20Actor _asbp_suckumm_c_3)))
                        (bind _asbp_suckumm_c_4 (Utilities|Casting|CastToBP_SuckUmm (Variables|Default|GetobjectToCheck)))
                        (Variables|/Game/Blueprints/BP_SuckUmm.BP_SuckUmm_C|SetParent%20Actor _returnvalue_2 _asbp_suckumm_c_4)
                        (Variables|/Game/Blueprints/BP_SuckUmm.BP_SuckUmm_C|SetChild%20Actor _asbp_suckumm_c_4 _returnvalue_2)))))))))))
    (:then_1
      ;[1 1 1] Respawn
      (if (Variables|Default|GetIs%20Respawning)
        (Utilities|FlowControl|Sequence
          (:then_0
            (Variables|Default|SetIs%20Respawning true))
          (:then_1
            (Utilities|Time|SetTimerbyEvent (delegate Custom|Set%20Alive) 3.0))
          (:then_2
            (Variables|Default|SetIs%20Dead false))
          (:then_3
            (Variables|/Script/Engine.PrimitiveComponent|SetbGenerateOverlapEvents (Variables|Default|GetSuck%20Collider) false))
          (:then_4
            (Variables|Default|SetCurrent%20Suck%20Level 0)))))
    (:then_2
      ;[1 1 1] Get Sucked
      (if (Variables|Default|GetIs%20Sucked)
        (bind _outactors (Actor|GetAllActorsOfClass "/Game/Blueprints/BP_PlayerCharacter.BP_PlayerCharacter_C"))
        (bind _array_element_3 (Utilities|Array|ForEachLoopwithBreak _outactors)
          (:LoopBody
            (if (!= _array_element_3 self)
              ;;[1 0 0] FIX THIS PLEASE
              (Transformation|SetActorLocation (+ _returnvalue (* (* (Math|Vector|Normalize (- (Transformation|GetActorLocation _array_element_3) _returnvalue)) (Utilities|Time|GetWorldDeltaSeconds)) (Variables|Default|GetSuck%20Speed))) false))))))))

(event Input|ActionEvents|InputActionJump
  ;[1 1 1] Double Jump
  (:Pressed
    (if (Math|Boolean|ANDBoolean (== (Variables|Default|GetCurrent%20Suck%20Level) 0) (not (Variables|Default|GetIs%20Sucked)) (not (Variables|Default|GetIs%20Stunned)))
      (bind _counter (Utilities|FlowControl|DoN 2)
        (:Exit
          (switch int _counter
            (:1
              (Character|Jump))
            (:2
              (Character|LaunchCharacter (Math|Vector|MakeVector 0.0 0.0 (Variables|/Script/Engine.CharacterMovementComponent|GetJumpZVelocity (Variables|Character|GetCharacterMovement))) false true))))))))

(event Input|ActionEvents|InputActionSuckMore
  ;[1 1 1] Suck Inputs
  (:Pressed
    (bind _counter (Utilities|FlowControl|DoN (Variables|Default|GetMax%20Suck%20Level))
      (:Exit
        (Variables|Default|SetCurrent%20Suck%20Level _counter)
        (CallFunction|SuckChanged)))))

(event Input|ActionEvents|InputActionThrow
  ;[1 1 1] Throw
  (:Pressed
    (Variables|Default|SetIs%20Throwing true))
  (:Released
    (Variables|Default|SetIs%20Throwing false)))

(event Input|ActionEvents|InputActionSuckLess
  ;[1 1 1] Suck Inputs
  (:Pressed
    (Utilities|FlowControl|Sequence
      (:then_0
        (Utilities|FlowControl|DoN (Variables|Default|GetMax%20Suck%20Level)) ; enters at Reset
      )
      (:then_1
        (Math|Integer|CompareInt (Variables|Default|GetCurrent%20Suck%20Level) 0
          (:>
            (Variables|Default|SetCurrent%20Suck%20Level (- (Variables|Default|GetCurrent%20Suck%20Level) 1))
            (CallFunction|SuckChanged)))))))

(event Input|AxisEvents|InputAxisMoveRight
  (params (AxisValue :type Float%20%28single-precision%29))
  ;[1 1 1] Movement
  (if (not (and (Variables|Default|GetIs%20Sucked) (Variables|Default|GetIs%20Stunned)))
    (Utilities|FlowControl|Sequence
      (:then_0
        ;[1 1 1] Look at rotation
        (Math|Float|CompareFloat AxisValue 0.0
          (:>
            (Pawn|SetControlRotation (Pawn|GetController) (Class|KismetMathLibrary|MakeRot 0.0 0.0 0.0)))
          (:<
            (Pawn|SetControlRotation (Pawn|GetController) (Class|KismetMathLibrary|MakeRot 0.0 1.8e+02 0.0)))))
      (:then_1
        (if (== (Variables|Default|GetCurrent%20Suck%20Level) 0)
          (Pawn|Input|AddMovementInput "1.000000,0.000000, 0" AxisValue false))))))

(fn ConstructionScript)